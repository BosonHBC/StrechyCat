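; Slope actor that gives a spinning BP_SpinTurtle a 1.5x boost to walk speed and jump velocity while overlapping it.
; BeginPlay binds SpeedUp and ResetSpeed to actor overlap begin and end, both acting only while the turtle is Rotating.
; SpeedUp caches original movement values on first use, and ResetSpeed restores them on exit, so a turtle that stops rotating before leaving keeps the boost.
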(event Custom|SpeedUp
  (params (OverlappedActor :type Actor%20Object%20Reference) (OtherActor :type Actor%20Object%20Reference))
  (bind _asbp_spin_turtle (Utilities|Casting|CastToBP_SpinTurtle OtherActor))
  (if (Variables|/Script/StretchyCat.SCSpinTurtle|GetbRotating _asbp_spin_turtle)
    (bind _ascharacter_movement_component (Utilities|Casting|CastToCharacterMovementComponent (Pawn|GetMovementComponent _asbp_spin_turtle)))
    (if (== (Variables|Default|GetOriginalWalkingSpeed) 0.0)
      (Variables|Default|SetOriginalWalkingSpeed (Variables|/Script/Engine.CharacterMovementComponent|GetMaxWalkSpeed _ascharacter_movement_component)))
    (Variables|/Script/Engine.CharacterMovementComponent|SetMaxWalkSpeed _ascharacter_movement_component (* (Variables|Default|GetOriginalWalkingSpeed) 1.5))
    (if (== (Variables|Default|GetOriginalJumpVelocity) 0.0)
      (Variables|Default|SetOriginalJumpVelocity (Variables|/Script/Engine.CharacterMovementComponent|GetJumpZVelocity _ascharacter_movement_component)))
    (Variables|/Script/Engine.CharacterMovementComponent|SetJumpZVelocity _ascharacter_movement_component (* (Variables|Default|GetOriginalJumpVelocity) 1.5))))

(event Custom|ResetSpeed
  (params (OverlappedActor :type Actor%20Object%20Reference) (OtherActor :type Actor%20Object%20Reference))
  (bind _originaljumpvelocity (Variables|Default|GetOriginalJumpVelocity))
  (bind _originalwalkingspeed (Variables|Default|GetOriginalWalkingSpeed))
  (bind _asbp_spin_turtle (Utilities|Casting|CastToBP_SpinTurtle OtherActor))
  (if (Variables|/Script/StretchyCat.SCSpinTurtle|GetbRotating _asbp_spin_turtle)
    (bind _ascharacter_movement_component (Utilities|Casting|CastToCharacterMovementComponent (Pawn|GetMovementComponent _asbp_spin_turtle)))
    (if (not (Math|Float|NearlyEqual(Float) _originaljumpvelocity 0.0 1e-06))
      (Variables|/Script/Engine.CharacterMovementComponent|SetJumpZVelocity _ascharacter_movement_component _originaljumpvelocity)
      (if (not (Math|Float|NearlyEqual(Float) _originalwalkingspeed 0.0 1e-06))
        (Variables|/Script/Engine.CharacterMovementComponent|SetMaxWalkSpeed _ascharacter_movement_component _originalwalkingspeed)))))

(event EventBeginPlay
  (EventDispatchers|BindEventtoOnActorBeginOverlap (delegate Custom|SpeedUp))
  (EventDispatchers|BindEventtoOnActorEndOverlap (delegate Custom|ResetSpeed)))

(event Collision|EventActorBeginOverlap
  (params (OtherActor :type Actor%20Object%20Reference)))

(event EventTick
  (params (DeltaSeconds :type Float%20%28single-precision%29)))

(fn ConstructionScript)