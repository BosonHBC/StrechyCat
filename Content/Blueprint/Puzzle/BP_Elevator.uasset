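; BP_Elevator is a puzzle elevator actor that moves between its starting location and a configured relative offset.
; While Moving is set, Tick steps it toward Destination at constant Speed, snapping into place within a distance threshold.
; With Loop set, each arrival reverses direction through SetDestinaton.
; MoveOnce and MoveBack trigger one-way trips by setting the destination and clearing Loop.
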(event EventBeginPlay
  (Variables|Default|SetOriginLocation (Transformation|GetActorLocation)))

(event Collision|EventActorBeginOverlap
  (params (OtherActor :type Actor%20Object%20Reference)))

(event EventTick
  (params (DeltaSeconds :type Float%20%28single-precision%29))
  (if (Variables|Default|GetbMoving)
    ;[1 1 1] Moving
    (bind _output_get (Variables|Default|SetDirection (Math|Vector|Normalize (- (Variables|Default|GetDestination) (Transformation|GetActorLocation)))))
    (Transformation|SetActorLocation (+ (Transformation|GetActorLocation) (* _output_get (* DeltaSeconds (Variables|Default|Getspeed)))) false false)
    (if (<= (Math|Vector|Distance(Vector) (Variables|Default|GetDestination) (Transformation|GetActorLocation)) (Variables|Default|GetdestThreoshold))
      (Variables|Default|SetbMoving false)
      (Transformation|SetActorLocation (Variables|Default|GetDestination) false false)
      (if (Variables|Default|GetbLoop)
        (if (Variables|Default|GetbGoUp)
          (CallFunction|SetDestinaton (Math|Vector|VectorZero))
          (Variables|Default|SetbGoUp false)
          (else
            (CallFunction|SetDestinaton (Variables|Default|GetRelativeUltimateLocation))
            (Variables|Default|SetbGoUp true)))))))

(fn ConstructionScript)

(fn SetDestinaton
  (params (Dest :type Vector))
  (Variables|Default|SetDestination (+ (Variables|Default|GetOriginLocation) Dest))
  (Variables|Default|SetbMoving true))

(fn MoveOnce
  (CallFunction|SetDestinaton (Variables|Default|GetRelativeUltimateLocation))
  (Variables|Default|SetbLoop false))

(fn MoveBack
  (CallFunction|SetDestinaton (Math|Vector|VectorZero))
  (Variables|Default|SetbLoop false))