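; BP_Container is a puzzle trigger that activates a linked elevator once enough objects enter its box.
; Overlaps by characters or BP_PickBox actors feed a duplicate-checked list and counter, which drives a progress percentage on a BP_ElevatorHint widget.
; At three, it moves the elevator and enables looping if off, with the authority then completing an uncompleted objective in the referenced room.
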(event OnComponentBeginOverlap(Box)
  (params (OverlappedComponent :type Primitive%20Component%20Object%20Reference) (OtherActor :type Actor%20Object%20Reference) (OtherComp :type Primitive%20Component%20Object%20Reference) (OtherBodyIndex :type Integer) (bFromSweep :type Boolean) (SweepResult :type Hit%20Result%20Structure%20%28by%20ref%29))
  (bind _ref_room (Variables|Default|GetRef_Room))
  (bind _insideactor (Variables|Default|GetInsideActor))
  (bind _returnvalue (Class|BaseRoom|GetAnUncompleteObjective _ref_room))
  (Utilities|Casting|CastToSCCharacterBase OtherActor
    (:then
      _)
    (:CastFailed
      (bind _asbp_pick_box (Utilities|Casting|CastToBP_PickBox OtherActor))))
  (if (not (Utilities|Array|ContainsItem _insideactor _asbp_pick_box))
    (Utilities|Array|AddUnique _insideactor _asbp_pick_box)
    (bind _result (Math|Integer|IncrementInt (Variables|Default|GetinsideCount))
      (:%20%20
        (bind _asbp_elevator_hint (Utilities|Casting|CastToBP_ElevatorHint (UserInterface|GetUserWidgetObject (Variables|Default|GetWidget))))
        (Default|SetPercentage _asbp_elevator_hint (/ (Math|Conversions|ToFloat(Integer) _result) 3.0))
        (if (>= _result 3)
          (bind _asbp_elevator (Utilities|Casting|CastToBP_Elevator (Variables|Default|GetElevator)))
          (Default|MoveOnce _asbp_elevator)
          (if (not (Variables|/Game/Blueprint/Puzzle/BP_Elevator.BP_Elevator_C|GetbLoop _asbp_elevator))
            (Variables|/Game/Blueprint/Puzzle/BP_Elevator.BP_Elevator_C|SetbLoop _asbp_elevator true)
            (Networking|SwitchHasAuthority
              (:Authority
                (Utilities|IsValid _returnvalue
                  (:Is%20Valid
                    (Class|ObjectiveItemBase|CompleteItself _returnvalue)))))))))))

(event EventBeginPlay)

(event Collision|EventActorBeginOverlap
  (params (OtherActor :type Actor%20Object%20Reference)))

(event EventTick
  (params (DeltaSeconds :type Float%20%28single-precision%29)))

(fn ConstructionScript)