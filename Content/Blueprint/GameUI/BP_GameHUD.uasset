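; BP_GameHUD is a HUD Blueprint that puts the main game UI on screen and shows short status messages.
; On BeginPlay it creates the GameMainUI widget, stores a reference and adds it to the viewport.
; ShowMessage writes text into that widget's Message field and sets a timer that calls ClearMessage to blank it shortly after.
; A CharacterSelect widget creation chain is left unconnected and never runs.
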(event Custom|ShowMessage
  (params (MessageToSend :type Text))
  (bind _gamemainui (Variables|Default|GetGameMainUI))
  (Utilities|IsValid _gamemainui
    (:Is%20Valid
      (Rendering|Components|TextRender|SetText (Variables|/Game/Blueprint/GameUI/GameMainUI.GameMainUI_C|GetMessage _gamemainui) MessageToSend)
      (Utilities|Time|SetTimerbyEvent (delegate Custom|ClearMessage) 2.0))))

(event Custom|ClearMessage
  (Rendering|Components|TextRender|SetText (Variables|/Game/Blueprint/GameUI/GameMainUI.GameMainUI_C|GetMessage (Variables|Default|GetGameMainUI)) ""))

(event EventBeginPlay
  (bind _returnvalue (UserInterface|CreateWidget "/Game/Blueprint/GameUI/GameMainUI.GameMainUI_C"))
  (Variables|Default|SetGameMainUI _returnvalue)
  (UserInterface|Viewport|AddtoViewport _returnvalue 0))

(fn ConstructionScript)