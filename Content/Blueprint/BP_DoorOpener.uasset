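; Interactable door opener actor that, on first interaction, moves itself, triggers its referenced door, and completes a room objective.
; Interaction starts movement toward an offset from its start location and calls MoveOnce on the door, then locks against reuse.
; It also completes an uncompleted objective from the referenced room for the interacting actor's SCBaseController.
; Tick steps it toward the destination at a fixed per-frame speed, not scaled by delta time, until within a small threshold.
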(event EventBeginPlay
  (Variables|Default|SetStartLocation (Transformation|GetActorLocation)))

(event Collision|EventActorBeginOverlap
  (params (OtherActor :type Actor%20Object%20Reference)))

(event EventTick
  (params (DeltaSeconds :type Float%20%28single-precision%29))
  (bind _returnvalue (Transformation|GetActorLocation))
  (if (not (Variables|Default|GetbArrived))
    (if (Variables|Default|GetbMoving)
      (Transformation|SetActorLocation (+ _returnvalue (* (Math|Vector|Normalize (- (Variables|Default|GetDestination) (Transformation|GetActorLocation))) (Variables|Default|Getspeed))) false false)
      (if (<= (Math|Vector|Distance(Vector) _returnvalue (Variables|Default|GetDestination)) 2.0)
        (Variables|Default|SetbArrived true)))))

(event EventOnDoInteractionBP
  (params (ownActor :type SC%20Character%20Base%20Object%20Reference))
  (bind _ref_dooe (Variables|Default|GetRef_Dooe))
  (bind _ref_room (Variables|Default|GetRef_Room))
  (bind _returnvalue (Class|BaseRoom|GetAnUncompleteObjective _ref_room))
  (if (not (Variables|Default|GetbDoorOpened))
    (CallFunction|StartMoving (Variables|Default|GetRelativeDest))
    (Default|MoveOnce _ref_dooe (Variables|/Game/Blueprint/Puzzle/BP_Elevator.BP_Elevator_C|GetbLoop _ref_dooe))
    (Variables|Default|SetbDoorOpened true)
    ;[1 1 1] Objective
    (bind _asscbase_controller (Utilities|Casting|CastToSCBaseController (Pawn|GetController ownActor)))
    (Utilities|IsValid _returnvalue
      (:Is%20Valid
        (Class|ObjectiveItemBase|CompleteObjective _returnvalue _asscbase_controller))
      (:Is%20Not%20Valid
        (Development|PrintString "No Obj Left")))))

(fn ConstructionScript)

(fn StartMoving
  (params (Destination :type Vector))
  (Variables|Default|SetDestination (+ Destination (Variables|Default|GetStartLocation)))
  (Variables|Default|SetbArrived false)
  (Variables|Default|SetbMoving true))