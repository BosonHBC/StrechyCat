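; StandOnObj is an objective actor that is completed by a character standing on it.
; On the authority, begin and end overlaps with an SCCharacterBase pass that character's SCBaseController to CompleteObjective and UncompleteObjective, printing a debug message if the controller cast fails.
; Tick polls the completion state and sets the text render to the complete or uncomplete text.
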(event Collision|EventActorBeginOverlap
  (params (OtherActor :type Actor%20Object%20Reference))
  (bind _assccharacter_base (Utilities|Casting|CastToSCCharacterBase OtherActor))
  (Networking|SwitchHasAuthority
    (:Authority
      (bind _asscbase_controller (Utilities|Casting|CastToSCBaseController (Pawn|GetController _assccharacter_base))
        (:then
          (Class|ObjectiveItemBase|CompleteObjective _asscbase_controller))
        (:CastFailed
          (Development|PrintString "CastFailed"))))))

(event Collision|EventActorEndOverlap
  (params (OtherActor :type Actor%20Object%20Reference))
  (bind _assccharacter_base (Utilities|Casting|CastToSCCharacterBase OtherActor))
  (Networking|SwitchHasAuthority
    (:Authority
      (bind _asscbase_controller (Utilities|Casting|CastToSCBaseController (Pawn|GetController _assccharacter_base))
        (:then
          (Class|ObjectiveItemBase|UncompleteObjective _asscbase_controller))
        (:CastFailed
          (Development|PrintString "CastFailed"))))))

(event EventTick
  (params (DeltaSeconds :type Float%20%28single-precision%29))
  (bind _textrender (Variables|Default|GetTextRender))
  (if (Class|ObjectiveItemBase|GetifCompleted)
    (Rendering|Components|TextRender|SetText _textrender (Variables|Default|GetCompleteText))
    (else
      (Rendering|Components|TextRender|SetText _textrender (Variables|Default|GetUncompleteText)))))

(fn ConstructionScript)